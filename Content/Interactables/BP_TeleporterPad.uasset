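; Interactable teleporter pad that sends the player to the destination point of a linked pad.
; Overlapping the trigger registers it as the player's interactable and shows a prompt.
; Interact freezes movement, shows HUD and VFX, waits, then moves the character, keeping rotation.
; The linked trigger's collision is disabled until its cooldown ends, preventing instant re-triggering, but IsTeleporting never clears, so each departure pad works once.
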(event `self.TriggerBox.OnComponentBeginOverlap`
  (params (OverlappedComponent :type "PrimitiveComponent Object Reference") (OtherActor :type "Actor Object Reference") (OtherComp :type "PrimitiveComponent Object Reference") (OtherBodyIndex :type Integer) (bFromSweep :type Boolean) (SweepResult :type "HitResult Structure (by ref)"))
  ; Overlap Detection - Cast & Validate
  (cast `Character` OtherActor)
  (if (and (and (not (`self.bIsTeleporting`)) (`KismetSystemLibrary.IsValid` (`self.LinkedTeleporter`))) (`self.bCanTeleport`))
    (`|ExecutionSequence`
      (:`then_0`
        (bind _asplayer_bp (cast `/Game/Player/Player_BP` OtherActor)))
      (:`then_1`
        (set `/Game/Player/Player_BP.CurrentInteractable` self _asplayer_bp)
        (bind _returnvalue (`|CreateWidget` (`self.InteractPromptWidgetClass`) (`GameplayStatics.GetPlayerController` 0)))
        (bind _output_get (set `self.PromptWidget` _returnvalue))
        (`UserWidget.AddToViewport` _output_get 0)))))

(event `/Game/Interfaces/BPI_Interactable.Interact`
  (params (Instigator :type "Character Object Reference"))
  (bind _promptwidget (`self.PromptWidget`))
  ; Teleport on Interact
  (if (and (and (not (`self.bIsTeleporting`)) (`KismetSystemLibrary.IsValid` (`self.LinkedTeleporter`))) (`self.bCanTeleport`))
    (`/Engine/EditorBlueprintResources/StandardMacros.IsValid` _promptwidget
      (:`Is Valid`
        (`Widget.RemoveFromParent` _promptwidget)
        (set `self.PromptWidget` null)
        (`self.StartTeleport` Instigator))
      (:`Is Not Valid`
        (`self.StartTeleport` Instigator)))))

(event `self.TriggerBox.OnComponentEndOverlap`
  (params (OverlappedComponent :type "PrimitiveComponent Object Reference") (OtherActor :type "Actor Object Reference") (OtherComp :type "PrimitiveComponent Object Reference") (OtherBodyIndex :type Integer))
  (bind _promptwidget (`self.PromptWidget`))
  ; Interact Prompt
  (bind _asplayer_bp (cast `/Game/Player/Player_BP` OtherActor))
  (set `/Game/Player/Player_BP.CurrentInteractable` null _asplayer_bp)
  (`/Engine/EditorBlueprintResources/StandardMacros.IsValid` _promptwidget
    (:`Is Valid`
      (`Widget.RemoveFromParent` _promptwidget)
      (set `self.PromptWidget` null))))

(event `StartTeleport`
  (params (TeleportingCharacter :type "Character Object Reference"))
  (bind _linkedteleporter (`self.LinkedTeleporter`))
  ; Execute Teleport Sequence
  (set `self.bIsTeleporting` true)
  (set `self.bCanTeleport` false)
  (`CharacterMovementComponent.SetMovementMode` (`Character.CharacterMovement` TeleportingCharacter) "MOVE_None" 0)
  (bind _returnvalue (`|CreateWidget` "/Game/UI/WBP_TeleportHUD.WBP_TeleportHUD_C" (`GameplayStatics.GetPlayerController` 0)))
  (bind _output_get (set `self.TeleportHUDWidget` _returnvalue))
  (`UserWidget.AddToViewport` _output_get 0)
  (`ActorComponent.Activate` (`self.TeleportVFX`) true)
  (`KismetSystemLibrary.Delay` (`self.TeleportDelay`))
  (`PrimitiveComponent.SetCollisionEnabled` (`self.GetComponentByClass` _linkedteleporter "/Script/Engine.BoxComponent") "NoCollision")
  (`self.ExecuteTeleport` TeleportingCharacter)
  (`Widget.RemoveFromParent` (`self.TeleportHUDWidget`))
  (`CharacterMovementComponent.SetMovementMode` (`Character.CharacterMovement` TeleportingCharacter) "MOVE_Walking" 0)
  (set `self.bIsTeleporting` true)
  (`self.ResetCooldown`)
  (`self.ResetCooldown` _linkedteleporter))

(event `ResetCooldown`
  ; Collision Cooldown
  (`KismetSystemLibrary.Delay` (`self.TeleportCooldown`))
  (set `self.bCanTeleport` true)
  (`PrimitiveComponent.SetCollisionEnabled` (`self.TriggerBox`) "QueryOnly"))

(fn `ExecuteTeleport`
  (params (TeleportingCharacter :type "Character Object Reference"))
  (bind _location (`self.GetDestinationLocation` (`self.LinkedTeleporter`)))
  (`self.K2_SetActorLocationAndRotation` TeleportingCharacter _location (`self.K2_GetActorRotation` TeleportingCharacter) false true)
  (`ActorComponent.Deactivate` (`self.TeleportVFX`)))

(fn `GetDestinationLocation`
  (returns (Location :type "Vector Structure"))
  (return (`SceneComponent.K2_GetComponentLocation` (`self.DestinationPoint`))))

(fn `UserConstructionScript`)