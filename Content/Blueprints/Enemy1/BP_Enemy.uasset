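; BP_Enemy is a ranged enemy that turns toward and attacks the player when its PawnSensing component sees a Player_BP.
; Each sighting rotates the actor to face the player and, if CanAttack is set, spawns a BP_Projectile at SpawnProjectile.
; Damage is applied directly to the player at the moment of firing, independent of any projectile hit.
; A short Delay resets CanAttack, limiting the fire rate.
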(event `self.ReceiveBeginPlay`)

(event `self.PawnSensing.OnSeePawn`
  (params (Pawn :type "Pawn Object Reference"))
  (bind _asplayer_bp (cast `/Game/Player/Player_BP` Pawn))
  (`self.K2_SetActorRotation` (`KismetMathLibrary.FindRelativeLookAtRotation` (`KismetMathLibrary.Conv_VectorToTransform` (`self.K2_GetActorLocation`)) (`self.K2_GetActorLocation` _asplayer_bp)))
  (if (`self.CanAttack?`)
    (`|SpawnActorFromClass` "/Game/Blueprints/Enemy1/BP_Projectile.BP_Projectile_C" (`SceneComponent.K2_GetComponentToWorld` (`self.SpawnProjectile`)) "Undefined" "MultiplyWithRoot" null null)
    (`GameplayStatics.ApplyDamage` _asplayer_bp 10.0)
    (set `self.CanAttack?` false)
    (`KismetSystemLibrary.Delay` 0.6)
    (set `self.CanAttack?` true)))

(fn `UserConstructionScript`)