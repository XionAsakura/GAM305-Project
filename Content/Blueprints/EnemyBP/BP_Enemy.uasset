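; BP_Enemy is an enemy Blueprint with a melee-style montage attack and simple damage handling.
; Attack plays the EnemyAttack montage on the mesh, using IsAttacking to block re-entry until the montage completes.
; AnyDamage subtracts damage from Health, then disables movement and destroys the actor only when Health equals exactly 50.
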(event `/Game/Blueprints/EnemyBP/BPI_Enemy.Attack`
  ; Attack
  (if (not (`self.isAttacking?`))
    (`|PlayMontage` (`self.Mesh`) "/Game/Blueprints/EnemyBP/EnemyAttack.EnemyAttack"
      (:`then`
        (set `self.isAttacking?` true))
      (:`OnCompleted`
        (set `self.isAttacking?` false)))))

(event `self.ReceiveAnyDamage`
  (params (Damage :type "Float (single-precision)") (DamageType :type "DamageType Object Reference") (InstigatedBy :type "Controller Object Reference") (DamageCauser :type "Actor Object Reference"))
  (set `self.health` (- (`self.health`) Damage))
  (if (== (`self.health`) 50.0)
    (`CharacterMovementComponent.DisableMovement` (`self.CharacterMovement`))
    (`self.K2_DestroyActor`)))

(fn `UserConstructionScript`)