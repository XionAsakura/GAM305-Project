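; AI controller for BP_Enemy that handles enemy patrolling, chasing the player and attacking.
; On possess it caches the enemy and starts a self-repeating patrol that picks a random nearby navigable point and calls AI MoveTo.
; Any perception update, with no stimulus check, starts an endless chase of player 0 that plays the virus attack montage on arrival and waits before repeating.
; Both behaviors are recursive event loops without a behavior tree.
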(event `Patrol`
  ; AI Patrol
  (`NavigationSystemV1.K2_GetRandomLocationInNavigableRadius` (`self.K2_GetActorLocation`) 400.0 null null :!label _label)
  (`|AIMoveTo` (`self.K2_GetPawn`) (0.0 0.0 0.0) null
    (:`OnSuccess`
      _)
    (:`OnFail`
      _))
  (`self.Patrol`))

(event `self.ReceivePossess`
  (params (PossessedPawn :type "Pawn Object Reference"))
  (bind _asbp_enemy (cast `/Game/Blueprints/EnemyBP/BP_Enemy` PossessedPawn))
  ; AI Patrol
  (set `self.AICharacter` _asbp_enemy)
  (goto _label))

(event `ChasePlayer`
  ; AI Follows Player + Attack
  (`|AIMoveTo` (`self.K2_GetPawn`) (0.0 0.0 0.0) (`GameplayStatics.GetPlayerCharacter` 0) :!label _label_2
    (:`OnSuccess`
      (bind _returnvalue (`Character.PlayAnimMontage` (`self.AICharacter`) "/Game/Blueprints/EnemyBP/VirusAttack_AnimMontage.VirusAttack_AnimMontage" 1.0 "None"))
      (`KismetSystemLibrary.Delay` _returnvalue))
    (:`OnFail`
      _))
  (`self.ChasePlayer`))

(event `self.AIPerception.OnTargetPerceptionUpdated`
  (params (Actor :type "Actor Object Reference") (Stimulus :type "AIStimulus Structure"))
  ; AI Follows Player + Attack
  (goto _label_2))

(fn `UserConstructionScript`)